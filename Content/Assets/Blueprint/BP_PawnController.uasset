(event EventBeginPlay
  (Setup|SetupImage)
  (Utilities|FlowControl|Delay 1.0)
  (CheckConditions|CheckConditions))

(fn ConstructionScript
  (Setup|SetupImage))

(fn SetupImage
  (bind _returnvalue (Rendering|Material|CreateDynamicMaterialInstance (Variables|Default|GetIcon) 0 (Utilities|Select :Index (Variables|ObjectsTypes|GetWordType) :NewEnumerator0 (Utilities|GetImageNouns) :NewEnumerator1 (Utilities|GetImageOperators) :NewEnumerator2 (Utilities|GetImageProperties) :NewEnumerator3 (Utilities|GetImageObjects)) "None" :!class /Script/Engine.PrimitiveComponent))
  (Variables|REF|SetMaterialDyn_REF _returnvalue))

(fn CheckConditions
  (switch Utilities|FlowControl|Switch|SwitchonEWordsType (Variables|ObjectsTypes|GetWordType)
    (:NewEnumerator0
      (CheckConditions|ResearchOperator))
    (:NewEnumerator1
      (CheckConditions|ConditionsOperator))
    (:NewEnumerator2
      (CheckConditions|ResearchOperator))
    (:NewEnumerator3
      (CheckConditions|ResearchOperator))))

(fn ConditionsOperator
  (bind _ref_around (Variables|REF|GetRef_Around))
  (bind _ref_around_2 (Variables|REF|GetRef_Around))
  (bind _output (Utilities|Array|Get(acopy) _ref_around_2 3))
  (bind _output_2 (Utilities|Array|Get(acopy) _ref_around 1))
  (bind _wordtype (Variables|BP_PawnController_C|GetWordType _output_2))
  (bind _wordtype_2 (Variables|BP_PawnController_C|GetWordType _output))
  (switch Utilities|FlowControl|Switch|SwitchonEOperators (Variables|ObjectsTypes|GetOperatorType)
    (:NewEnumerator0
      (Check|GetAround)
      (for (_array_element _array_index) (Variables|REF|GetRef_Around)
        (Utilities|IsValid _array_element
          (:Is%20Valid
            (if (Utilities|Enum|Equal(Enum) (Variables|BP_PawnController_C|GetWordType _array_element) "NewEnumerator0")
              (LocalVariables|SetNounsTypes (Variables|BP_PawnController_C|GetNounsType _array_element))
              (switch int _array_index
                (:0
                  (Utilities|IsValid _output_2
                    (:Is%20Valid
                      (if (Utilities|Enum|Equal(Enum) _wordtype "NewEnumerator2")
                        (LocalVariables|SetPropertiesTypes (Variables|BP_PawnController_C|GetPropertiesType _output_2))
                        (Logic|IsLogic (LocalVariables|GetNounsTypes) (LocalVariables|GetPropertiesTypes) :!label _label)
                        (elif (Utilities|Enum|Equal(Enum) _wordtype "NewEnumerator0")
                          (LocalVariables|SetNounsHitTypes (Variables|BP_PawnController_C|GetNounsType _output_2))
                          (Logic|IsLogicwithNouns (LocalVariables|GetNounsTypes) (LocalVariables|GetNounsHitTypes) :!label _label_2))))))
                (:2
                  (Utilities|IsValid _output
                    (:Is%20Valid
                      (if (Utilities|Enum|Equal(Enum) _wordtype_2 "NewEnumerator2")
                        (LocalVariables|SetPropertiesTypes (Variables|BP_PawnController_C|GetPropertiesType _output))
                        (goto _label)
                        (elif (Utilities|Enum|Equal(Enum) _wordtype_2 "NewEnumerator0")
                          (LocalVariables|SetNounsHitTypes (Variables|BP_PawnController_C|GetNounsType _output))
                          (goto _label_2))))))))))))))

(fn CheckAround
  (bind _returnvalue (Transformation|GetActorLocation))
  (bind _returnvalue_2 (Transformation|GetActorLocation))
  (bind _returnvalue_3 (Transformation|GetActorLocation))
  (bind _returnvalue_4 (Transformation|GetActorLocation))
  (Utilities|FlowControl|Sequence
    (:then_0
      (bind _outhit (Collision|LineTraceByChannel _returnvalue (+ _returnvalue (* (Math|Vector|GetRightVector (Transformation|GetActorRotation)) -1e+02)) "TraceTypeQuery1" false 0 "None"))
      (LocalVariables|SetUpHit _outhit))
    (:then_1
      (bind _outhit_2 (Collision|LineTraceByChannel _returnvalue_3 (+ _returnvalue_3 (* (Math|Vector|GetRightVector (Transformation|GetActorRotation)) 1e+02)) "TraceTypeQuery1" false 0 "None"))
      (LocalVariables|SetDownHit _outhit_2))
    (:then_2
      (bind _outhit_3 (Collision|LineTraceByChannel _returnvalue_2 (+ _returnvalue_2 (* (Math|Vector|GetForwardVector (Transformation|GetActorRotation)) -1e+02)) "TraceTypeQuery1" false 0 "None"))
      (LocalVariables|SetLeftHit _outhit_3))
    (:then_3
      (bind _outhit_4 (Collision|LineTraceByChannel _returnvalue_4 (+ _returnvalue_4 (* (Math|Vector|GetForwardVector (Transformation|GetActorRotation)) 1e+02)) "TraceTypeQuery1" false 0 "None"))
      (LocalVariables|SetRightHit _outhit_4))
    (:then_4
      (return (Utilities|Array|MakeArray (LocalVariables|GetUpHit) (LocalVariables|GetDownHit) (LocalVariables|GetLeftHit) (LocalVariables|GetRightHit))))))

(fn GetAround
  (for (_array_element _array_index) (Check|CheckAround)
    (if (.bblockinghit _array_element)
      (Utilities|IsValid (.AsBP%20Pawn%20Controller (Utilities|Casting|CastToBP_PawnController (.hitactor _array_element)))
        (:Is%20Valid
          (Utilities|Array|SetArrayElem (Variables|REF|GetRef_Around) _array_index (.AsBP%20Pawn%20Controller (Utilities|Casting|CastToBP_PawnController (.hitactor _array_element)))))
        (:Is%20Not%20Valid
          (Check|CheckRemoveConditions _array_index :!label _label)
          (Utilities|Array|SetArrayElem (Variables|REF|GetRef_Around) _array_index 0)))
      (else
        (goto _label)))))

(fn IsLogic
  (params (NounsInput :type ENouns%20Enum :default "NewEnumerator0") (PropertiesInput :type EProperties%20Enum :default "NewEnumerator0"))
  (LocalVariables|SetNounsLocal NounsInput)
  (LocalVariables|SetPropertiesLocal PropertiesInput)
  (Development|PrintText (Utilities|Text|FormatText "Nouns : {A} 
Properties : {B}" (Utilities|String|EnumtoString (LocalVariables|GetNounsLocal)) (Utilities|String|EnumtoString (LocalVariables|GetPropertiesLocal))))
  (switch Utilities|FlowControl|Switch|SwitchonEProperties (LocalVariables|GetPropertiesLocal)
    (:NewEnumerator0
      (bind _array_element (Utilities|CheckGoodObject (LocalVariables|GetNounsLocal))
        (:true
          (Variables|BP_PawnController_C|SetIsDefeat _array_element true))))
    (:NewEnumerator1
      (bind _array_element_2 (Utilities|CheckGoodObject (LocalVariables|GetNounsLocal))
        (:true
          (Variables|BP_PawnController_C|SetIsFloat _array_element_2 true)
          (Rendering|Material|SetScalarParameterValue (Variables|BP_PawnController_C|GetMaterialDyn_REF _array_element_2) "IsFloat" 1.0 :!class /Script/Engine.MaterialInstanceDynamic))))
    (:NewEnumerator2
      (bind _array_element_3 (Utilities|CheckGoodObject (LocalVariables|GetNounsLocal))
        (:true
          (Variables|BP_PawnController_C|SetIsHot _array_element_3 true))))
    (:NewEnumerator3
      (bind _array_element_4 (Utilities|CheckGoodObject (LocalVariables|GetNounsLocal))
        (:true
          (Variables|BP_PawnController_C|SetIsMelt _array_element_4 true))))
    (:NewEnumerator4
      (bind _array_element_5 (Utilities|CheckGoodObject (LocalVariables|GetNounsLocal))
        (:true
          (Variables|BP_PawnController_C|SetIsMove _array_element_5 true))))
    (:NewEnumerator5
      (bind _array_element_6 (Utilities|CheckGoodObject (LocalVariables|GetNounsLocal))
        (:true
          (Variables|BP_PawnController_C|SetIsOpen _array_element_6 true))))
    (:NewEnumerator6
      (bind _array_element_7 (Utilities|CheckGoodObject (LocalVariables|GetNounsLocal))
        (:true
          (Variables|BP_PawnController_C|SetIsPush _array_element_7 true))))
    (:NewEnumerator7
      (bind _array_element_8 (Utilities|CheckGoodObject (LocalVariables|GetNounsLocal))
        (:true
          (Variables|BP_PawnController_C|SetIsShut _array_element_8 true))))
    (:NewEnumerator8
      (bind _array_element_9 (Utilities|CheckGoodObject (LocalVariables|GetNounsLocal))
        (:true
          (Variables|BP_PawnController_C|SetIsSink _array_element_9 true))))
    (:NewEnumerator9
      (bind _array_element_10 (Utilities|CheckGoodObject (LocalVariables|GetNounsLocal))
        (:true
          (Variables|BP_PawnController_C|SetIsStop _array_element_10 true))))
    (:NewEnumerator10
      (bind _array_element_11 (Utilities|CheckGoodObject (LocalVariables|GetNounsLocal))
        (:true
          (Variables|BP_PawnController_C|SetIsWeak _array_element_11 true))))
    (:NewEnumerator11
      (bind _array_element_12 (Utilities|CheckGoodObject (LocalVariables|GetNounsLocal))
        (:true
          (Variables|BP_PawnController_C|SetIsWin _array_element_12 true))))
    (:NewEnumerator12
      (LocalVariables|SetPCLocal (.AsPC%20Custom%20Controller (Utilities|Casting|CastToPC_CustomController (Game|GetPlayerController 0))))
      (bind _outactors (Actor|GetAllActorsOfClass "BP_PawnController_C"))
      (for _array_element_13 _outactors
        (if (Utilities|Enum|Equal(Enum) (Variables|BP_PawnController_C|GetWordType _array_element_13) "NewEnumerator3")
          (if (Utilities|Enum|Equal(Enum) (Variables|BP_PawnController_C|GetNounsType _array_element_13) (LocalVariables|GetNounsLocal))
            (Default|AddPossessPawn (LocalVariables|GetPCLocal) _array_element_13)))))))

(fn IsLogicwithNouns
  (params (NounsInput :type ENouns%20Enum :default "NewEnumerator0") (NounsHitInput :type ENouns%20Enum :default "NewEnumerator0"))
  (LocalVariables|SetNounsLocal NounsInput)
  (LocalVariables|SetNounsHitLocal NounsHitInput)
  (Development|PrintText (Utilities|Text|FormatText "Nouns : {A} 
Properties : {B}" (Utilities|String|EnumtoString (LocalVariables|GetNounsLocal)) (Utilities|String|EnumtoString (LocalVariables|GetNounsHitLocal))))
  (bind _outactors (Actor|GetAllActorsOfClass "BP_PawnController_C"))
  (for _array_element _outactors
    (if (Utilities|Enum|Equal(Enum) (Variables|BP_PawnController_C|GetWordType _array_element) "NewEnumerator3")
      (if (Utilities|Enum|Equal(Enum) (Variables|BP_PawnController_C|GetNounsType _array_element) (LocalVariables|GetNounsHitLocal))
        (Variables|BP_PawnController_C|SetNounsType _array_element (LocalVariables|GetNounsLocal))
        (Setup|SetupImage _array_element)
        (Default|RemovePossessPawn (.AsPC%20Custom%20Controller (Utilities|Casting|CastToPC_CustomController (Game|GetPlayerController 0))) _array_element)))))

(fn CheckCanMove
  (params (Direction :type Integer))
  (bind _arrayhit (Check|CheckAround))
  (bind _output (Utilities|Array|Get(acopy) _arrayhit Direction))
  (bind _asbp_pawn_controller (Utilities|Casting|CastToBP_PawnController (.hitactor _output)))
  (Utilities|IsValid (.hitactor _output)
    (:Is%20Valid
      (return (and (not (Variables|BP_PawnController_C|GetIsBlock _asbp_pawn_controller)) (not (Variables|BP_PawnController_C|GetIsStop _asbp_pawn_controller)))))
    (:Is%20Not%20Valid
      (return (not (.bblockinghit _output))))))

(fn CallMove
  (CheckConditions|CheckConditions))

(fn ResearchOperator
  (Check|GetAround)
  (for _array_element (Variables|REF|GetRef_Around)
    (Utilities|IsValid _array_element
      (:Is%20Valid
        (if (Utilities|Enum|Equal(Enum) (Variables|BP_PawnController_C|GetWordType _array_element) "NewEnumerator1")
          (Logic|CallMove _array_element))))))

(fn CheckRemoveConditions
  (params (ID :type Integer))
  (bind _returnvalue (Utilities|Select :Index ID :Option%200 1 :Option%201 0 :Option%202 3 :Option%203 2))
  (bind _ref_around (Variables|REF|GetRef_Around))
  (bind _ref_around_2 (Variables|REF|GetRef_Around))
  (bind _output (Utilities|Array|Get(acopy) _ref_around ID))
  (bind _output_2 (Utilities|Array|Get(acopy) _ref_around_2 _returnvalue))
  (Utilities|IsValid _output
    (:Is%20Valid
      (bind _output_get (LocalVariables|SetWordType1Local (Variables|BP_PawnController_C|GetWordType _output)))
      (if (Utilities|Enum|NotEqual(Enum) _output_get "NewEnumerator1")
        (LocalVariables|SetNounsType1Local (Variables|BP_PawnController_C|GetNounsType _output))
        (LocalVariables|SetPropertiesType1Local (Variables|BP_PawnController_C|GetPropertiesType _output))
        (Utilities|IsValid _output_2
          (:Is%20Valid
            (bind _output_get_2 (LocalVariables|SetWordType2Local (Variables|BP_PawnController_C|GetWordType _output_2)))
            (if (Utilities|Enum|NotEqual(Enum) _output_get_2 "NewEnumerator1")
              (LocalVariables|SetNounsType2Local (Variables|BP_PawnController_C|GetNounsType _output_2))
              (LocalVariables|SetPropertiesType2Local (Variables|BP_PawnController_C|GetPropertiesType _output_2))
              (LocalVariables|SetREF_PC (.AsPC%20Custom%20Controller (Utilities|Casting|CastToPC_CustomController (Game|GetPlayerController 0))))
              (bind _outactors (Actor|GetAllActorsOfClass "BP_PawnController_C"))
              (for _array_element _outactors
                (if (Utilities|Enum|Equal(Enum) (Variables|BP_PawnController_C|GetWordType _array_element) "NewEnumerator3")
                  (if (Utilities|Enum|Equal(Enum) (Variables|BP_PawnController_C|GetNounsType _array_element) (LocalVariables|GetNounsType1Local))
                    (switch Utilities|FlowControl|Switch|SwitchonEProperties (LocalVariables|GetPropertiesType2Local)
                      (:NewEnumerator0
                        (Variables|BP_PawnController_C|SetIsDefeat _array_element false))
                      (:NewEnumerator1
                        (Rendering|Material|SetScalarParameterValue (Variables|BP_PawnController_C|GetMaterialDyn_REF _array_element) "IsFloat" 0.0 :!class /Script/Engine.MaterialInstanceDynamic)
                        (Variables|BP_PawnController_C|SetIsFloat _array_element false))
                      (:NewEnumerator2
                        (Variables|BP_PawnController_C|SetIsHot _array_element false))
                      (:NewEnumerator3
                        (Variables|BP_PawnController_C|SetIsMelt _array_element false))
                      (:NewEnumerator4
                        (Variables|BP_PawnController_C|SetIsMove _array_element false))
                      (:NewEnumerator5
                        (Variables|BP_PawnController_C|SetIsOpen _array_element false))
                      (:NewEnumerator6
                        (Variables|BP_PawnController_C|SetIsPush _array_element false))
                      (:NewEnumerator7
                        (Variables|BP_PawnController_C|SetIsShut _array_element false))
                      (:NewEnumerator8
                        (Variables|BP_PawnController_C|SetIsSink _array_element false))
                      (:NewEnumerator9
                        (Variables|BP_PawnController_C|SetIsStop _array_element false))
                      (:NewEnumerator10
                        (Variables|BP_PawnController_C|SetIsWeak _array_element false))
                      (:NewEnumerator11
                        (Variables|BP_PawnController_C|SetIsWin _array_element false))
                      (:NewEnumerator12
                        (Default|RemovePossessPawn (LocalVariables|GetREF_PC) _array_element)))))))))))))