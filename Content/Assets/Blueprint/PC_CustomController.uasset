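; Player controller for a grid-based word-rule puzzle game, steering every BP_PawnController in PossessedPawn at once.
; Each move input line-traces ahead, letting CheckPawn resolve property interactions like destruction, blocking or winning via UW_Win.
; MoveText then gathers the chain of pushable actors by repeated traces, and PushActor shifts it one 100-unit cell if unblocked.
; Pawns step afterwards, ignoring diagonal input; rewind, idle and pause inputs are empty.
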(event Input|EnhancedActionEvents|EnhancedInputActionIA_Rewind
  (params (ActionValue :type Boolean) (ElapsedSeconds :type Float%20%28double-precision%29) (TriggeredSeconds :type Float%20%28double-precision%29) (InputAction :type Input%20Action%20Object%20Reference :default "/Game/Assets/Blueprint/Input/Actions/IA_Rewind.IA_Rewind")))

(event Input|EnhancedActionEvents|EnhancedInputActionIA_Move
  (params (ActionValue :type Vector%202D%20Structure) (ElapsedSeconds :type Float%20%28double-precision%29) (TriggeredSeconds :type Float%20%28double-precision%29) (InputAction :type Input%20Action%20Object%20Reference :default "/Game/Assets/Blueprint/Input/Actions/IA_Move.IA_Move"))
  (bind (_x _y) (Math|Vector2D|BreakVector2D ActionValue))
  (:Started
    (for _array_element (Variables|Default|GetPossessed%20Pawn)
      (bind _cancontinue (Logic|MoveText _array_element ActionValue))
      (if _cancontinue
        (Utilities|IsValid _array_element
          (:Is%20Valid
            (if (Default|CheckCanMove (.AsBP%20Pawn%20Controller (Utilities|Casting|CastToBP_PawnController _array_element)) (Logic|GetDirection ActionValue))
              (if (Logic|DisableAngle ActionValue) :!label _label
                (Transformation|SetActorLocation _array_element (Math|Vector|MakeVector (+ (.x (Transformation|GetActorLocation _array_element)) (* _x 1e+02)) (+ (.y (Transformation|GetActorLocation _array_element)) (* _y 1e+02)) (.z (Transformation|GetActorLocation _array_element))) false false))
              (elif (Variables|/Game/Assets/Blueprint/BP_PawnController.BP_PawnController_C|GetIsFloat (.AsBP%20Pawn%20Controller (Utilities|Casting|CastToBP_PawnController _array_element)))
                (goto _label)))))))))

(event Input|EnhancedActionEvents|EnhancedInputActionIA_Idle
  (params (ActionValue :type Boolean) (ElapsedSeconds :type Float%20%28double-precision%29) (TriggeredSeconds :type Float%20%28double-precision%29) (InputAction :type Input%20Action%20Object%20Reference :default "/Game/Assets/Blueprint/Input/Actions/IA_Idle.IA_Idle")))

(event Input|EnhancedActionEvents|EnhancedInputActionIA_Pause
  (params (ActionValue :type Boolean) (ElapsedSeconds :type Float%20%28double-precision%29) (TriggeredSeconds :type Float%20%28double-precision%29) (InputAction :type Input%20Action%20Object%20Reference :default "/Game/Assets/Blueprint/Input/Actions/IA_Pause.IA_Pause")))

(event EventBeginPlay
  (bind _returnvalue (PlayerController|LocalPlayerSubsystems|GetEnhancedInputLocalPlayerSubsystem))
  (Utilities|IsValid _returnvalue
    (:Is%20Valid
      (Input|AddMappingContext _returnvalue "/Game/Assets/Blueprint/Input/IMC_PlayerInput.IMC_PlayerInput" 0 "(bIgnoreAllPressedKeysUntilRelease=True,bForceImmediately=False,bNotifyUserSettings=False)")
      (Variables|Default|SetbShowMouseCursor false))))

(fn ConstructionScript)

(fn AddPossessPawn
  (params (NewPawn :type Pawn%20Object%20Reference))
  (Pawn|Possess NewPawn)
  (Utilities|Array|AddUnique (Variables|Default|GetPossessed%20Pawn) NewPawn))

(fn RemovePossessPawn
  (params (RmPawn :type Pawn%20Object%20Reference))
  (Utilities|Array|RemoveItem (Variables|Default|GetPossessed%20Pawn) RmPawn))

(fn CheckPawn
  (params (Pawn :type Pawn%20Object%20Reference) (CurrentPawn :type Pawn%20Object%20Reference))
  (bind _asbp_pawn_controller (Utilities|Casting|CastToBP_PawnController Pawn))
  (bind _asbp_pawn_controller_2 (Utilities|Casting|CastToBP_PawnController CurrentPawn))
  (Utilities|IsValid Pawn
    (:Is%20Valid
      (Utilities|IsValid CurrentPawn
        (:Is%20Valid
          (if (and (Variables|/Game/Assets/Blueprint/BP_PawnController.BP_PawnController_C|GetIsHot _asbp_pawn_controller) (Variables|/Game/Assets/Blueprint/BP_PawnController.BP_PawnController_C|GetIsMelt _asbp_pawn_controller_2))
            _
            (elif (and (not (Variables|/Game/Assets/Blueprint/BP_PawnController.BP_PawnController_C|GetIsStop _asbp_pawn_controller)) (Variables|/Game/Assets/Blueprint/BP_PawnController.BP_PawnController_C|GetIsWeak _asbp_pawn_controller_2))
              _
              (elif (and (and (Utilities|Enum|Equal(Enum) (Variables|/Game/Assets/Blueprint/BP_PawnController.BP_PawnController_C|GetWordType _asbp_pawn_controller) "NewEnumerator3") (Utilities|Enum|Equal(Enum) (Variables|/Game/Assets/Blueprint/BP_PawnController.BP_PawnController_C|GetNounsType _asbp_pawn_controller) "NewEnumerator6")) (Variables|/Game/Assets/Blueprint/BP_PawnController.BP_PawnController_C|GetIsOpen _asbp_pawn_controller_2))
                _
                (elif (and (Variables|/Game/Assets/Blueprint/BP_PawnController.BP_PawnController_C|GetIsSink _asbp_pawn_controller) (Variables|/Game/Assets/Blueprint/BP_PawnController.BP_PawnController_C|GetIsMelt _asbp_pawn_controller_2))
                  _
                  (else
                    (if (Variables|/Game/Assets/Blueprint/BP_PawnController.BP_PawnController_C|GetIsWeak _asbp_pawn_controller_2)
                      _
                      (elif (Variables|/Game/Assets/Blueprint/BP_PawnController.BP_PawnController_C|GetIsHot _asbp_pawn_controller)
                        _
                        (elif (Variables|/Game/Assets/Blueprint/BP_PawnController.BP_PawnController_C|GetIsDefeat _asbp_pawn_controller)
                          _
                          (elif (Variables|/Game/Assets/Blueprint/BP_PawnController.BP_PawnController_C|GetIsSink _asbp_pawn_controller)
                            _
                            (elif (Variables|/Game/Assets/Blueprint/BP_PawnController.BP_PawnController_C|GetIsWeak _asbp_pawn_controller)
                              (Actor|DestroyActor _asbp_pawn_controller)
                              (return false)
                              (elif (Variables|/Game/Assets/Blueprint/BP_PawnController.BP_PawnController_C|GetIsWin _asbp_pawn_controller)
                                (CallFunction|SetWin)
                                (return false)
                                (elif (and (Utilities|Enum|Equal(Enum) (Variables|/Game/Assets/Blueprint/BP_PawnController.BP_PawnController_C|GetWordType _asbp_pawn_controller) "NewEnumerator3") (not (Variables|/Game/Assets/Blueprint/BP_PawnController.BP_PawnController_C|GetIsPush _asbp_pawn_controller)))
                                  (return false)
                                  (else
                                    (return true)))))))))
                    (Actor|DestroyActor _asbp_pawn_controller_2)
                    (CallFunction|RemovePossessPawn _asbp_pawn_controller_2)
                    (return false))))))
          (Actor|DestroyActor _asbp_pawn_controller)
          (Actor|DestroyActor _asbp_pawn_controller_2)
          (CallFunction|RemovePossessPawn _asbp_pawn_controller_2)
          (return false))))))

(fn GetDirection
  (params (2DAxis :type Vector%202D%20Structure))
  (if (>= (.x 2DAxis) 1.0)
    (bind _output_get (LocalVariables|SetDirectionLocal 3))
    (return _output_get)
    (elif (<= (.x 2DAxis) -1.0)
      (bind _output_get_2 (LocalVariables|SetDirectionLocal 2))
      (return _output_get_2)
      (elif (>= (.y 2DAxis) 1.0)
        (bind _output_get_3 (LocalVariables|SetDirectionLocal 1))
        (return _output_get_3)
        (elif (<= (.y 2DAxis) -1.0)
          (bind _output_get_4 (LocalVariables|SetDirectionLocal 0))
          (return _output_get_4))))))

(fn DisableAngle
  (params (Axis :type Vector%202D%20Structure))
  (return (not (and (or (>= (.x Axis) 0.1) (<= (.x Axis) -0.1)) (or (>= (.y Axis) 0.1) (<= (.y Axis) -0.1))))))

(fn MoveText
  (params (Actor :type Actor%20Object%20Reference) (2DVector :type Vector%202D%20Structure))
  (bind _index (LocalVariables|GetIndex))
  (bind _actorlist (LocalVariables|GetActorList))
  (bind _index_2 (LocalVariables|GetIndex))
  (bind _actorlist_2 (LocalVariables|GetActorList))
  (bind _index_3 (LocalVariables|GetIndex))
  (bind _actorlist_3 (LocalVariables|GetActorList))
  (bind _index_4 (LocalVariables|GetIndex))
  (bind _actorlist_4 (LocalVariables|GetActorList))
  (bind _output (Utilities|Array|Get(acopy) _actorlist_4 _index))
  (bind _output_2 (Utilities|Array|Get(acopy) _actorlist _index_2))
  (bind _output_3 (Utilities|Array|Get(acopy) _actorlist_2 _index_3))
  (bind _output_4 (Utilities|Array|Get(acopy) _actorlist_3 _index_4))
  (bind _returnvalue (Transformation|GetActorLocation _output))
  (bind _returnvalue_2 (Transformation|GetActorLocation _output_2))
  (bind _returnvalue_3 (Transformation|GetActorLocation _output_3))
  (bind _returnvalue_4 (Transformation|GetActorLocation _output_4))
  (bind _output_get (LocalVariables|SetActorSelected Actor))
  (if (not (Variables|/Game/Assets/Blueprint/BP_PawnController.BP_PawnController_C|GetIsFloat (.AsBP%20Pawn%20Controller (Utilities|Casting|CastToBP_PawnController _output_get))))
    (if (>= (.x 2DVector) 1.0)
      (LocalVariables|SetDirection "Right")
      (elif (<= (.x 2DVector) -1.0)
        (LocalVariables|SetDirection "Left")
        (elif (>= (.y 2DVector) 1.0)
          (LocalVariables|SetDirection "Down")
          (elif (<= (.y 2DVector) -1.0)
            (LocalVariables|SetDirection "Up")
            (else
              (return true))))))
    (switch string (LocalVariables|GetDirection)
      (:Up
        (bind (_outhit _returnvalue_5) (Collision|LineTraceByChannel (Transformation|GetActorLocation (LocalVariables|GetActorSelected)) (+ (Transformation|GetActorLocation (LocalVariables|GetActorSelected)) (* (Math|Vector|GetRightVector (Transformation|GetActorRotation (LocalVariables|GetActorSelected))) -1e+02)) "TraceTypeQuery1" false (Variables|Default|GetPossessed%20Pawn) "None"))
        (if _returnvalue_5
          (Utilities|IsValid (.HitActor (Collision|BreakHitResult _outhit))
            (:Is%20Valid
              (bind _cancontinue (CallFunction|CheckPawn (.AsBP%20Pawn%20Controller (Utilities|Casting|CastToBP_PawnController (.HitActor (Collision|BreakHitResult _outhit)))) (.AsBP%20Pawn%20Controller (Utilities|Casting|CastToBP_PawnController (LocalVariables|GetActorSelected)))))
              (if _cancontinue
                (if (Math|Boolean|ANDBoolean (not (Variables|/Game/Assets/Blueprint/BP_PawnController.BP_PawnController_C|GetIsBlock (.AsBP%20Pawn%20Controller (Utilities|Casting|CastToBP_PawnController (.HitActor (Collision|BreakHitResult _outhit)))))) (not (Variables|/Game/Assets/Blueprint/BP_PawnController.BP_PawnController_C|GetIsStop (.AsBP%20Pawn%20Controller (Utilities|Casting|CastToBP_PawnController (.HitActor (Collision|BreakHitResult _outhit)))))) (not (Variables|/Game/Assets/Blueprint/BP_PawnController.BP_PawnController_C|GetIsFloat (.AsBP%20Pawn%20Controller (Utilities|Casting|CastToBP_PawnController (.HitActor (Collision|BreakHitResult _outhit)))))))
                  (Utilities|Array|Add (LocalVariables|GetActorList) (.HitActor (Collision|BreakHitResult _outhit)))
                  (while (and (not (LocalVariables|GetIsEmpty)) (not (LocalVariables|GetIsBlock)))
                    (Utilities|IsValid _output
                      (:Is%20Valid
                        (bind (_outhit_2 _returnvalue_6) (Collision|LineTraceByChannel _returnvalue (+ _returnvalue (* (Math|Vector|GetRightVector (Transformation|GetActorRotation _output)) -1e+02)) "TraceTypeQuery1" false (LocalVariables|GetActorList) "None"))
                        (if _returnvalue_6
                          (if (Math|Boolean|ANDBoolean (not (Variables|/Game/Assets/Blueprint/BP_PawnController.BP_PawnController_C|GetIsBlock (.AsBP%20Pawn%20Controller (Utilities|Casting|CastToBP_PawnController (.HitActor (Collision|BreakHitResult _outhit_2)))))) (not (Variables|/Game/Assets/Blueprint/BP_PawnController.BP_PawnController_C|GetIsStop (.AsBP%20Pawn%20Controller (Utilities|Casting|CastToBP_PawnController (.HitActor (Collision|BreakHitResult _outhit_2)))))) (not (Variables|/Game/Assets/Blueprint/BP_PawnController.BP_PawnController_C|GetIsFloat (.AsBP%20Pawn%20Controller (Utilities|Casting|CastToBP_PawnController (.HitActor (Collision|BreakHitResult _outhit_2)))))))
                            (if (Utilities|Enum|NotEqual(Enum) (Variables|/Game/Assets/Blueprint/BP_PawnController.BP_PawnController_C|GetWordType (.AsBP%20Pawn%20Controller (Utilities|Casting|CastToBP_PawnController (.HitActor (Collision|BreakHitResult _outhit_2))))) "NewEnumerator3")
                              (Utilities|Array|Add (LocalVariables|GetActorList) (.AsBP%20Pawn%20Controller (Utilities|Casting|CastToBP_PawnController (.HitActor (Collision|BreakHitResult _outhit_2)))) :!label _label)
                              (Math|Integer|IncrementInt (LocalVariables|GetIndex))
                              (elif (Variables|/Game/Assets/Blueprint/BP_PawnController.BP_PawnController_C|GetIsPush (.AsBP%20Pawn%20Controller (Utilities|Casting|CastToBP_PawnController (.HitActor (Collision|BreakHitResult _outhit_2)))))
                                (goto _label)
                                (else
                                  (LocalVariables|SetIsBlock true))))
                            (else
                              (LocalVariables|SetIsBlock true)))
                          (else
                            (LocalVariables|SetIsEmpty true))))
                      (:Is%20Not%20Valid
                        (LocalVariables|SetIsEmpty true))))
                  (if (not (LocalVariables|GetIsBlock))
                    (Logic|PushActor (LocalVariables|GetActorList) (LocalVariables|GetDirection))
                    (return true)
                    (else
                      (return false))))))
            (:Is%20Not%20Valid
              (return true)))
          (else
            (return true))))
      (:Down
        (bind (_outhit_3 _returnvalue_7) (Collision|LineTraceByChannel (Transformation|GetActorLocation (LocalVariables|GetActorSelected)) (+ (Transformation|GetActorLocation (LocalVariables|GetActorSelected)) (* (Math|Vector|GetRightVector (Transformation|GetActorRotation (LocalVariables|GetActorSelected))) 1e+02)) "TraceTypeQuery1" false (Variables|Default|GetPossessed%20Pawn) "None"))
        (if _returnvalue_7
          (Utilities|IsValid (.HitActor (Collision|BreakHitResult _outhit_3))
            (:Is%20Valid
              (bind _cancontinue_2 (CallFunction|CheckPawn (.AsBP%20Pawn%20Controller (Utilities|Casting|CastToBP_PawnController (.HitActor (Collision|BreakHitResult _outhit_3)))) (.AsBP%20Pawn%20Controller (Utilities|Casting|CastToBP_PawnController (LocalVariables|GetActorSelected)))))
              (if _cancontinue_2
                (if (Math|Boolean|ANDBoolean (not (Variables|/Game/Assets/Blueprint/BP_PawnController.BP_PawnController_C|GetIsBlock (.AsBP%20Pawn%20Controller (Utilities|Casting|CastToBP_PawnController (.HitActor (Collision|BreakHitResult _outhit_3)))))) (not (Variables|/Game/Assets/Blueprint/BP_PawnController.BP_PawnController_C|GetIsStop (.AsBP%20Pawn%20Controller (Utilities|Casting|CastToBP_PawnController (.HitActor (Collision|BreakHitResult _outhit_3)))))) (not (Variables|/Game/Assets/Blueprint/BP_PawnController.BP_PawnController_C|GetIsFloat (.AsBP%20Pawn%20Controller (Utilities|Casting|CastToBP_PawnController (.HitActor (Collision|BreakHitResult _outhit_3)))))))
                  (Utilities|Array|Add (LocalVariables|GetActorList) (.HitActor (Collision|BreakHitResult _outhit_3)))
                  (while (and (not (LocalVariables|GetIsEmpty)) (not (LocalVariables|GetIsBlock)))
                    (Utilities|IsValid _output_4
                      (:Is%20Valid
                        (bind (_outhit_4 _returnvalue_8) (Collision|LineTraceByChannel _returnvalue_4 (+ _returnvalue_4 (* (Math|Vector|GetRightVector (Transformation|GetActorRotation _output_4)) 1e+02)) "TraceTypeQuery1" false (LocalVariables|GetActorList) "None"))
                        (if _returnvalue_8
                          (if (Math|Boolean|ANDBoolean (not (Variables|/Game/Assets/Blueprint/BP_PawnController.BP_PawnController_C|GetIsBlock (.AsBP%20Pawn%20Controller (Utilities|Casting|CastToBP_PawnController (.HitActor (Collision|BreakHitResult _outhit_4)))))) (not (Variables|/Game/Assets/Blueprint/BP_PawnController.BP_PawnController_C|GetIsStop (.AsBP%20Pawn%20Controller (Utilities|Casting|CastToBP_PawnController (.HitActor (Collision|BreakHitResult _outhit_4)))))) (not (Variables|/Game/Assets/Blueprint/BP_PawnController.BP_PawnController_C|GetIsFloat (.AsBP%20Pawn%20Controller (Utilities|Casting|CastToBP_PawnController (.HitActor (Collision|BreakHitResult _outhit_4)))))))
                            (if (Utilities|Enum|NotEqual(Enum) (Variables|/Game/Assets/Blueprint/BP_PawnController.BP_PawnController_C|GetWordType (.AsBP%20Pawn%20Controller (Utilities|Casting|CastToBP_PawnController (.HitActor (Collision|BreakHitResult _outhit_4))))) "NewEnumerator3")
                              (Utilities|Array|Add (LocalVariables|GetActorList) (.AsBP%20Pawn%20Controller (Utilities|Casting|CastToBP_PawnController (.HitActor (Collision|BreakHitResult _outhit_4)))) :!label _label_2)
                              (Math|Integer|IncrementInt (LocalVariables|GetIndex))
                              (elif (Variables|/Game/Assets/Blueprint/BP_PawnController.BP_PawnController_C|GetIsPush (.AsBP%20Pawn%20Controller (Utilities|Casting|CastToBP_PawnController (.HitActor (Collision|BreakHitResult _outhit_4)))))
                                (goto _label_2)
                                (else
                                  (LocalVariables|SetIsBlock true))))
                            (else
                              (LocalVariables|SetIsBlock true)))
                          (else
                            (LocalVariables|SetIsEmpty true))))
                      (:Is%20Not%20Valid
                        (LocalVariables|SetIsEmpty true))))
                  (if (not (LocalVariables|GetIsBlock))
                    (Logic|PushActor (LocalVariables|GetActorList) (LocalVariables|GetDirection))
                    (return true)
                    (else
                      (return false))))))
            (:Is%20Not%20Valid
              (return true)))
          (else
            (return true))))
      (:Left
        (bind (_outhit_5 _returnvalue_9) (Collision|LineTraceByChannel (Transformation|GetActorLocation (LocalVariables|GetActorSelected)) (+ (Transformation|GetActorLocation (LocalVariables|GetActorSelected)) (* (Math|Vector|GetForwardVector (Transformation|GetActorRotation (LocalVariables|GetActorSelected))) -1e+02)) "TraceTypeQuery1" false (Variables|Default|GetPossessed%20Pawn) "None"))
        (if _returnvalue_9
          (Utilities|IsValid (.HitActor (Collision|BreakHitResult _outhit_5))
            (:Is%20Valid
              (bind _cancontinue_3 (CallFunction|CheckPawn (.AsBP%20Pawn%20Controller (Utilities|Casting|CastToBP_PawnController (.HitActor (Collision|BreakHitResult _outhit_5)))) (.AsBP%20Pawn%20Controller (Utilities|Casting|CastToBP_PawnController (LocalVariables|GetActorSelected)))))
              (if _cancontinue_3
                (if (Math|Boolean|ANDBoolean (not (Variables|/Game/Assets/Blueprint/BP_PawnController.BP_PawnController_C|GetIsBlock (.AsBP%20Pawn%20Controller (Utilities|Casting|CastToBP_PawnController (.HitActor (Collision|BreakHitResult _outhit_5)))))) (not (Variables|/Game/Assets/Blueprint/BP_PawnController.BP_PawnController_C|GetIsStop (.AsBP%20Pawn%20Controller (Utilities|Casting|CastToBP_PawnController (.HitActor (Collision|BreakHitResult _outhit_5)))))) (not (Variables|/Game/Assets/Blueprint/BP_PawnController.BP_PawnController_C|GetIsFloat (.AsBP%20Pawn%20Controller (Utilities|Casting|CastToBP_PawnController (.HitActor (Collision|BreakHitResult _outhit_5)))))))
                  (Utilities|Array|Add (LocalVariables|GetActorList) (.HitActor (Collision|BreakHitResult _outhit_5)))
                  (while (and (not (LocalVariables|GetIsEmpty)) (not (LocalVariables|GetIsBlock)))
                    (Utilities|IsValid _output_3
                      (:Is%20Valid
                        (bind (_outhit_6 _returnvalue_10) (Collision|LineTraceByChannel _returnvalue_3 (+ _returnvalue_3 (* (Math|Vector|GetForwardVector (Transformation|GetActorRotation _output_3)) -1e+02)) "TraceTypeQuery1" false (LocalVariables|GetActorList) "None"))
                        (if _returnvalue_10
                          (if (Math|Boolean|ANDBoolean (not (Variables|/Game/Assets/Blueprint/BP_PawnController.BP_PawnController_C|GetIsBlock (.AsBP%20Pawn%20Controller (Utilities|Casting|CastToBP_PawnController (.HitActor (Collision|BreakHitResult _outhit_6)))))) (not (Variables|/Game/Assets/Blueprint/BP_PawnController.BP_PawnController_C|GetIsStop (.AsBP%20Pawn%20Controller (Utilities|Casting|CastToBP_PawnController (.HitActor (Collision|BreakHitResult _outhit_6)))))) (not (Variables|/Game/Assets/Blueprint/BP_PawnController.BP_PawnController_C|GetIsFloat (.AsBP%20Pawn%20Controller (Utilities|Casting|CastToBP_PawnController (.HitActor (Collision|BreakHitResult _outhit_6)))))))
                            (if (Utilities|Enum|NotEqual(Enum) (Variables|/Game/Assets/Blueprint/BP_PawnController.BP_PawnController_C|GetWordType (.AsBP%20Pawn%20Controller (Utilities|Casting|CastToBP_PawnController (.HitActor (Collision|BreakHitResult _outhit_6))))) "NewEnumerator3")
                              (Utilities|Array|Add (LocalVariables|GetActorList) (.AsBP%20Pawn%20Controller (Utilities|Casting|CastToBP_PawnController (.HitActor (Collision|BreakHitResult _outhit_6)))) :!label _label_3)
                              (Math|Integer|IncrementInt (LocalVariables|GetIndex))
                              (elif (Variables|/Game/Assets/Blueprint/BP_PawnController.BP_PawnController_C|GetIsPush (.AsBP%20Pawn%20Controller (Utilities|Casting|CastToBP_PawnController (.HitActor (Collision|BreakHitResult _outhit_6)))))
                                (goto _label_3)
                                (else
                                  (LocalVariables|SetIsBlock true))))
                            (else
                              (LocalVariables|SetIsBlock true)))
                          (else
                            (LocalVariables|SetIsEmpty true))))
                      (:Is%20Not%20Valid
                        (LocalVariables|SetIsEmpty true))))
                  (if (not (LocalVariables|GetIsBlock))
                    (Logic|PushActor (LocalVariables|GetActorList) (LocalVariables|GetDirection))
                    (return true)
                    (else
                      (return false))))))
            (:Is%20Not%20Valid
              (return true)))
          (else
            (return true))))
      (:Right
        (bind (_outhit_7 _returnvalue_11) (Collision|LineTraceByChannel (Transformation|GetActorLocation (LocalVariables|GetActorSelected)) (+ (Transformation|GetActorLocation (LocalVariables|GetActorSelected)) (* (Math|Vector|GetForwardVector (Transformation|GetActorRotation (LocalVariables|GetActorSelected))) 1e+02)) "TraceTypeQuery1" false (Variables|Default|GetPossessed%20Pawn) "None"))
        (if _returnvalue_11
          (Utilities|IsValid (.HitActor (Collision|BreakHitResult _outhit_7))
            (:Is%20Valid
              (bind _cancontinue_4 (CallFunction|CheckPawn (.AsBP%20Pawn%20Controller (Utilities|Casting|CastToBP_PawnController (.HitActor (Collision|BreakHitResult _outhit_7)))) (.AsBP%20Pawn%20Controller (Utilities|Casting|CastToBP_PawnController (LocalVariables|GetActorSelected)))))
              (if _cancontinue_4
                (if (Math|Boolean|ANDBoolean (not (Variables|/Game/Assets/Blueprint/BP_PawnController.BP_PawnController_C|GetIsBlock (.AsBP%20Pawn%20Controller (Utilities|Casting|CastToBP_PawnController (.HitActor (Collision|BreakHitResult _outhit_7)))))) (not (Variables|/Game/Assets/Blueprint/BP_PawnController.BP_PawnController_C|GetIsStop (.AsBP%20Pawn%20Controller (Utilities|Casting|CastToBP_PawnController (.HitActor (Collision|BreakHitResult _outhit_7)))))) (not (Variables|/Game/Assets/Blueprint/BP_PawnController.BP_PawnController_C|GetIsFloat (.AsBP%20Pawn%20Controller (Utilities|Casting|CastToBP_PawnController (.HitActor (Collision|BreakHitResult _outhit_7)))))))
                  (Utilities|Array|Add (LocalVariables|GetActorList) (.HitActor (Collision|BreakHitResult _outhit_7)))
                  (while (and (not (LocalVariables|GetIsEmpty)) (not (LocalVariables|GetIsBlock)))
                    (Utilities|IsValid _output_2
                      (:Is%20Valid
                        (bind (_outhit_8 _returnvalue_12) (Collision|LineTraceByChannel _returnvalue_2 (+ _returnvalue_2 (* (Math|Vector|GetForwardVector (Transformation|GetActorRotation _output_2)) 1e+02)) "TraceTypeQuery1" false (LocalVariables|GetActorList) "None"))
                        (if _returnvalue_12
                          (if (Math|Boolean|ANDBoolean (not (Variables|/Game/Assets/Blueprint/BP_PawnController.BP_PawnController_C|GetIsBlock (.AsBP%20Pawn%20Controller (Utilities|Casting|CastToBP_PawnController (.HitActor (Collision|BreakHitResult _outhit_8)))))) (not (Variables|/Game/Assets/Blueprint/BP_PawnController.BP_PawnController_C|GetIsStop (.AsBP%20Pawn%20Controller (Utilities|Casting|CastToBP_PawnController (.HitActor (Collision|BreakHitResult _outhit_8)))))) (not (Variables|/Game/Assets/Blueprint/BP_PawnController.BP_PawnController_C|GetIsFloat (.AsBP%20Pawn%20Controller (Utilities|Casting|CastToBP_PawnController (.HitActor (Collision|BreakHitResult _outhit_8)))))))
                            (if (Utilities|Enum|NotEqual(Enum) (Variables|/Game/Assets/Blueprint/BP_PawnController.BP_PawnController_C|GetWordType (.AsBP%20Pawn%20Controller (Utilities|Casting|CastToBP_PawnController (.HitActor (Collision|BreakHitResult _outhit_8))))) "NewEnumerator3")
                              (Utilities|Array|Add (LocalVariables|GetActorList) (.AsBP%20Pawn%20Controller (Utilities|Casting|CastToBP_PawnController (.HitActor (Collision|BreakHitResult _outhit_8)))) :!label _label_4)
                              (Math|Integer|IncrementInt (LocalVariables|GetIndex))
                              (elif (Variables|/Game/Assets/Blueprint/BP_PawnController.BP_PawnController_C|GetIsPush (.AsBP%20Pawn%20Controller (Utilities|Casting|CastToBP_PawnController (.HitActor (Collision|BreakHitResult _outhit_8)))))
                                (goto _label_4)
                                (else
                                  (LocalVariables|SetIsBlock true))))
                            (else
                              (LocalVariables|SetIsBlock true)))
                          (else
                            (LocalVariables|SetIsEmpty true))))
                      (:Is%20Not%20Valid
                        (LocalVariables|SetIsEmpty true))))
                  (if (not (LocalVariables|GetIsBlock))
                    (Logic|PushActor (LocalVariables|GetActorList) (LocalVariables|GetDirection))
                    (return true)
                    (else
                      (return false))))))
            (:Is%20Not%20Valid
              (return true)))
          (else
            (return true)))))))

(fn PushActor
  (params (ActorListToPush :type Array%20of%20Actor%20Object%20References) (Direction :type String))
  (LocalVariables|SetActorToPush ActorListToPush)
  (switch string Direction
    (:Up
      (for _array_element (LocalVariables|GetActorToPush)
        (Transformation|SetActorLocation _array_element (Math|Vector|MakeVector (.x (Transformation|GetActorLocation _array_element)) (+ (.y (Transformation|GetActorLocation _array_element)) -1e+02) (.z (Transformation|GetActorLocation _array_element))) true false)
        (Default|CallMove (.AsBP%20Pawn%20Controller (Utilities|Casting|CastToBP_PawnController _array_element)))))
    (:Down
      (for _array_element_2 (LocalVariables|GetActorToPush)
        (Transformation|SetActorLocation _array_element_2 (Math|Vector|MakeVector (.x (Transformation|GetActorLocation _array_element_2)) (+ (.y (Transformation|GetActorLocation _array_element_2)) 1e+02) (.z (Transformation|GetActorLocation _array_element_2))) true false)
        (Default|CallMove (.AsBP%20Pawn%20Controller (Utilities|Casting|CastToBP_PawnController _array_element_2)))))
    (:Left
      (for _array_element_3 (LocalVariables|GetActorToPush)
        (Transformation|SetActorLocation _array_element_3 (Math|Vector|MakeVector (+ (.x (Transformation|GetActorLocation _array_element_3)) -1e+02) (.y (Transformation|GetActorLocation _array_element_3)) (.z (Transformation|GetActorLocation _array_element_3))) true false)
        (Default|CallMove (.AsBP%20Pawn%20Controller (Utilities|Casting|CastToBP_PawnController _array_element_3)))))
    (:Right
      (for _array_element_4 (LocalVariables|GetActorToPush)
        (Transformation|SetActorLocation _array_element_4 (Math|Vector|MakeVector (+ (.x (Transformation|GetActorLocation _array_element_4)) 1e+02) (.y (Transformation|GetActorLocation _array_element_4)) (.z (Transformation|GetActorLocation _array_element_4))) true false)
        (Default|CallMove (.AsBP%20Pawn%20Controller (Utilities|Casting|CastToBP_PawnController _array_element_4)))))))

(fn RemoveAllPossessPawn
  (Utilities|Array|Clear (Variables|Default|GetPossessed%20Pawn)))

(fn SetWin
  (bind _returnvalue (UserInterface|CreateWidget "/Game/Assets/Blueprint/Canvas/UW_Win.UW_Win_C"))
  (UserInterface|Viewport|AddtoViewport _returnvalue 0)
  (CallFunction|RemoveAllPossessPawn)
  (Variables|Default|SetbShowMouseCursor true))